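; Big door actor that opens once the first-person player has touched all three of its key collision volumes.
; Each key overlap fires only once, setting its flag and switching its matching light to the active material.
; When all three flags are set, the door mesh is hidden and loses collision.
; The Death function resets the flags and lights and restores the door's visibility and collision.
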(event `self.KeyCollision1.OnComponentBeginOverlap`
  (params (OverlappedComponent :type "PrimitiveComponent Object Reference") (OtherActor :type "Actor Object Reference") (OtherComp :type "PrimitiveComponent Object Reference") (OtherBodyIndex :type Integer) (bFromSweep :type Boolean) (SweepResult :type "HitResult Structure (by ref)"))
  (bind _door (`self.Door`))
  (if (not (`self.1kEY`))
    (cast `/Game/FirstPerson/Blueprints/BP_FirstPersonCharacter` OtherActor)
    (set `self.1kEY` true)
    (`PrimitiveComponent.SetMaterial` (`self.Light1`) 0 "/Game/Material/M_active.M_active")
    (if (and (`self.1kEY`) (`self.2kEY`) (`self.3kEY`)) :!label _label
      (`PrimitiveComponent.SetCollisionEnabled` _door "NoCollision")
      (`SceneComponent.SetVisibility` _door false false))))

(event `self.KeyCollision2.OnComponentBeginOverlap`
  (params (OverlappedComponent :type "PrimitiveComponent Object Reference") (OtherActor :type "Actor Object Reference") (OtherComp :type "PrimitiveComponent Object Reference") (OtherBodyIndex :type Integer) (bFromSweep :type Boolean) (SweepResult :type "HitResult Structure (by ref)"))
  (if (not (`self.2kEY`))
    (cast `/Game/FirstPerson/Blueprints/BP_FirstPersonCharacter` OtherActor)
    (set `self.2kEY` true)
    (`PrimitiveComponent.SetMaterial` (`self.Light2`) 0 "/Game/Material/M_active.M_active")
    (goto _label)))

(event `self.KeyCollision3.OnComponentBeginOverlap`
  (params (OverlappedComponent :type "PrimitiveComponent Object Reference") (OtherActor :type "Actor Object Reference") (OtherComp :type "PrimitiveComponent Object Reference") (OtherBodyIndex :type Integer) (bFromSweep :type Boolean) (SweepResult :type "HitResult Structure (by ref)"))
  (if (not (`self.3kEY`))
    (cast `/Game/FirstPerson/Blueprints/BP_FirstPersonCharacter` OtherActor)
    (set `self.3kEY` true)
    (`PrimitiveComponent.SetMaterial` (`self.Light3`) 0 "/Game/Material/M_active.M_active")
    (goto _label)))

(fn `Death`
  (bind _door (`self.Door`))
  (set `self.1kEY` false)
  (set `self.2kEY` false)
  (set `self.3kEY` false)
  (`PrimitiveComponent.SetMaterial` (`self.Light3`) 0 "/Game/Material/M_Inactive.M_Inactive")
  (`PrimitiveComponent.SetMaterial` (`self.Light2`) 0 "/Game/Material/M_Inactive.M_Inactive")
  (`PrimitiveComponent.SetMaterial` (`self.Light1`) 0 "/Game/Material/M_Inactive.M_Inactive")
  (`SceneComponent.SetVisibility` _door true false)
  (`PrimitiveComponent.SetCollisionEnabled` _door "QueryAndPhysics"))

(fn `UserConstructionScript`)