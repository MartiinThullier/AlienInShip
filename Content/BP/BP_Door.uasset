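; BP_Door is an automatic vertically moving door that opens when the player or BP_Menace enters its trigger box.
; Opening reports a long-range "sound" noise event for AI, plays a sound at world origin and runs a timeline lerping the mesh's Z between closed and open points.
; A recursive delay rechecks every few seconds, reversing the timeline to close once the player leaves, regardless of BP_Menace.
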(event `self.Box.OnComponentBeginOverlap`
  (params (OverlappedComponent :type "PrimitiveComponent Object Reference") (OtherActor :type "Actor Object Reference") (OtherComp :type "PrimitiveComponent Object Reference") (OtherBodyIndex :type Integer) (bFromSweep :type Boolean) (SweepResult :type "HitResult Structure (by ref)"))
  (if (or (== OtherActor (`GameplayStatics.GetPlayerCharacter` 0)) (== OtherActor "/Game/BP/BP_Menace.BP_Menace"))
    (if (not (or (`self.DoorIsMoving`) (`self.IsOpened`)))
      (set `self.DoorIsMoving` true)
      (`AISense_Hearing.ReportNoiseEvent` (`SceneComponent.K2_GetComponentLocation` (`self.DefaultSceneRoot`)) 1.0 self 400000.0 "sound")
      (`self.DoorAction` true)
      (`self.DoorCloseTimer`))))

(event `DoorCloseTimer`
  (`KismetSystemLibrary.Delay` 3.0)
  (if (`PrimitiveComponent.IsOverlappingActor` (`self.Box`) (`GameplayStatics.GetPlayerCharacter` 0))
    (`self.DoorCloseTimer`)
    (else
      (`self.DoorAction` false))))

(event `DoorAction`
  (params (`OpenDoor?` :type Boolean))
  (bind _doorasset (`self.DoorAsset`))
  (bind (_returnvalue_x _returnvalue_y) (`KismetMathLibrary.BreakVector` (`SceneComponent.K2_GetComponentLocation` _doorasset)))
  (bind (_returnvalue_x_2 _returnvalue_y_2 _returnvalue_z) (`KismetMathLibrary.BreakVector` (`SceneComponent.K2_GetComponentLocation` (`self.DoorOpenPoint`))))
  (bind (_returnvalue_x_3 _returnvalue_y_3 _returnvalue_z_2) (`KismetMathLibrary.BreakVector` (`SceneComponent.K2_GetComponentLocation` (`self.DoorClosePoint`))))
  (`GameplayStatics.PlaySoundAtLocation` "/Game/sounds/DoorSFX.DoorSFX" (0.0 0.0 0.0) (struct) 2.0 1.0 0.0 null null null null)
  (if `OpenDoor?`
    (set `self.IsOpened` true)
    (bind (_direction _doormovement) (`Timeline|Door` :!via `PlayFromStart` :!label _label)
      (:`Update`
        (`SceneComponent.K2_SetWorldLocation` _doorasset (`KismetMathLibrary.MakeVector` _returnvalue_x _returnvalue_y (`KismetMathLibrary.Lerp` _returnvalue_z_2 _returnvalue_z _doormovement)) false false))
      (:`Finished`
        (set `self.DoorIsMoving` false)))
    (else
      (set `self.IsOpened` false)
      (goto _label :!via `ReverseFromEnd`))))

(fn `UserConstructionScript`)