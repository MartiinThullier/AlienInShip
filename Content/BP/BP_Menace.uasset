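; BP_Menace is an AI enemy that patrols random targets in one of two zone lists, chosen by IsMathys.
; AI Perception interrupts patrol: sound triggers faster investigation, other stimuli trigger a still faster player chase.
; Forgetting the player restores patrol speed and resumes wandering.
; For differently tagged destinations, it walks to the nearest BP_Vent linking both areas, teleports to the bound vent, and adopts the new area tag.
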(event `OnTargetPerceptionForgotten_Event`
  (params (Actor :type "Actor Object Reference"))
  (bind _returnvalue (`KismetMathLibrary.Vector_Distance` (`self.K2_GetActorLocation` (`self.TempAct`)) (`self.K2_GetActorLocation` self)))
  (cast `/Game/FirstPerson/Blueprints/BP_FirstPersonCharacter` Actor)
  (set `CharacterMovementComponent.MaxWalkSpeed` 300.0 (`self.CharacterMovement`))
  (if (`self.IsMathys`) :!label _label
    (bind _output_get (set `self.target` (`KismetArrayLibrary.Array_Random` (`self.ZoneMathys`))))
    (if (`self.ActorHasTag` _output_get (`self.Tag`))
      (`|AIMoveTo` self (0.0 0.0 0.0) (`self.target`) :!label _label_2
        (:`OnSuccess`
          (`KismetSystemLibrary.Delay` 1.0)
          (goto _label)))
      (else
        _))
    (else
      (bind _output_get_2 (set `self.target` (`KismetArrayLibrary.Array_Random` (`self.ZoneElio`))))
      (if (`self.ActorHasTag` _output_get_2 (`self.Tag`))
        (goto _label_2)
        (else
          _))))
  (bind _outactors (`GameplayStatics.GetAllActorsOfClass` "/Game/BP/BP_Vent.BP_Vent_C"))
  (for _array_element _outactors
    (set `self.TempAct` _array_element)
    (if (`self.ActorHasTag` (`self.TempAct`) (`self.Tag`))
      (if (`self.ActorHasTag` (`/Game/BP/BP_Vent.BoundVent` (`self.TempAct`)) (`|GetArrayItem` (`Actor.Tags` (`self.target`))))
        (if (`KismetSystemLibrary.IsValid` (`self.closestVent`))
          (if (< _returnvalue (`self.dist`))
            (set `self.dist` _returnvalue)
            (set `self.closestVent` (`self.TempAct`)))
          (else
            (bind _output_get_3 (set `self.closestVent` (`self.TempAct`)))
            (set `self.dist` (`KismetMathLibrary.Vector_Distance` (`self.K2_GetActorLocation` _output_get_3) (`self.K2_GetActorLocation` self))))))))
  (`|AIMoveTo` self (0.0 0.0 0.0) (`self.closestVent`) 20.0
    (:`OnSuccess`
      (bind _asbp_vent (cast `/Game/BP/BP_Vent` (`self.closestVent`)))
      (`self.K2_SetActorLocation` (`self.K2_GetActorLocation` (`/Game/BP/BP_Vent.BoundVent` _asbp_vent)))
      (set `self.Tag` (`|GetArrayItem` (`Actor.Tags` (`self.target`))))
      (`|AIMoveTo` self (0.0 0.0 0.0) (`self.target`)
        (:`OnSuccess`
          (set `self.closestVent` null)
          (`KismetSystemLibrary.Delay` 1.0)
          (`KismetSystemLibrary.PrintString` "ALAIDE")
          (`self.Restart`))))))

(event `self.ReceiveBeginPlay`
  (add `AIPerceptionComponent.OnTargetPerceptionForgotten` (`self.AIPerception`) (delegate `OnTargetPerceptionForgotten_Event`))
  (`KismetSystemLibrary.PrintString` (`KismetStringLibrary.Conv_NameToString` (`self.Tag`)))
  (goto _label))

(event `Restart`
  (goto _label))

(event `self.AIPerception.OnTargetPerceptionUpdated`
  (params (Actor :type "Actor Object Reference") (Stimulus :type "AIStimulus Structure"))
  (bind _returnvalue (`KismetMathLibrary.Vector_Distance` (`self.K2_GetActorLocation` (`self.TempAct`)) (`self.K2_GetActorLocation` self)))
  (`KismetSystemLibrary.PrintString` "Hello")
  (if (not (== Stimulus_Tag "sound"))
    (bind _asbp_first_person_character (cast `/Game/FirstPerson/Blueprints/BP_FirstPersonCharacter` Actor))
    (set `CharacterMovementComponent.MaxWalkSpeed` 700.0 (`self.CharacterMovement`))
    (`|AIMoveTo` self (0.0 0.0 0.0) _asbp_first_person_character)
    (else
      (set `CharacterMovementComponent.MaxWalkSpeed` 600.0 (`self.CharacterMovement`))
      (set `self.SoundStimulusLoc` Stimulus_StimulusLocation)
      (if (`self.ActorHasTag` Actor (`self.Tag`))
        (`|AIMoveTo` self (`self.SoundStimulusLoc`) null
          (:`OnSuccess`
            (`KismetSystemLibrary.Delay` 1.0)
            (set `CharacterMovementComponent.MaxWalkSpeed` 300.0 (`self.CharacterMovement`))
            (`self.Restart`)))
        (else
          (bind _outactors (`GameplayStatics.GetAllActorsOfClass` "/Game/BP/BP_Vent.BP_Vent_C"))
          (for _array_element _outactors
            (set `self.TempAct` _array_element)
            (if (`self.ActorHasTag` (`self.TempAct`) (`self.Tag`))
              (if (`self.ActorHasTag` (`/Game/BP/BP_Vent.BoundVent` (`self.TempAct`)) (`|GetArrayItem` (`Actor.Tags` Actor)))
                (if (`KismetSystemLibrary.IsValid` (`self.closestVent`))
                  (if (< _returnvalue (`self.dist`))
                    (set `self.dist` _returnvalue)
                    (set `self.closestVent` (`self.TempAct`)))
                  (else
                    (bind _output_get (set `self.closestVent` (`self.TempAct`)))
                    (set `self.dist` (`KismetMathLibrary.Vector_Distance` (`self.K2_GetActorLocation` _output_get) (`self.K2_GetActorLocation` self))))))))
          (`|AIMoveTo` self (0.0 0.0 0.0) (`self.closestVent`) 20.0
            (:`OnSuccess`
              (`KismetSystemLibrary.PrintString` "cool")
              (bind _asbp_vent (cast `/Game/BP/BP_Vent` (`self.closestVent`)))
              (`self.K2_SetActorLocation` (`self.K2_GetActorLocation` (`/Game/BP/BP_Vent.BoundVent` _asbp_vent)))
              (set `self.Tag` (`|GetArrayItem` (`Actor.Tags` Actor)))
              (`|AIMoveTo` self (`self.SoundStimulusLoc`) null
                (:`OnSuccess`
                  (set `CharacterMovementComponent.MaxWalkSpeed` 300.0 (`self.CharacterMovement`))
                  (set `self.closestVent` null)
                  (`KismetSystemLibrary.Delay` 1.0)
                  (`self.Restart`))))))))))

(fn `UserConstructionScript`)