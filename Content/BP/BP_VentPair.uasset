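; BP_VentPair is a container actor that links two BP_Vent child actors, BPVent and BPVent1, into a connected pair.
; On BeginPlay it sets each vent's BoundVent to the other, so the two reference each other.
; It also copies the first component tag of each child actor component onto its spawned vent, passing per-instance tags down to the actors.
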(event `self.ReceiveBeginPlay`
  (bind _bp_vent (`self.BP_Vent`))
  (bind _bp_vent1 (`self.BP_Vent1`))
  (bind _childactor (`ChildActorComponent.ChildActor` (`self.BP_Vent1`)))
  (bind _childactor_2 (`ChildActorComponent.ChildActor` (`self.BP_Vent`)))
  (bind _asbp_vent (cast `/Game/BP/BP_Vent` _childactor))
  (set `/Game/BP/BP_Vent.BoundVent` _childactor_2 _asbp_vent)
  (bind _asbp_vent_2 (cast `/Game/BP/BP_Vent` _childactor_2))
  (set `/Game/BP/BP_Vent.BoundVent` _childactor _asbp_vent_2)
  (bind _asbp_vent_3 (cast `/Game/BP/BP_Vent` (`ChildActorComponent.ChildActor` _bp_vent1)))
  (`KismetArrayLibrary.Array_Add` (`Actor.Tags` _asbp_vent_3) (`|GetArrayItem` (`ActorComponent.ComponentTags` _bp_vent1)))
  (bind _asbp_vent_4 (cast `/Game/BP/BP_Vent` (`ChildActorComponent.ChildActor` _bp_vent)))
  (`KismetArrayLibrary.Array_Add` (`Actor.Tags` _asbp_vent_4) (`|GetArrayItem` (`ActorComponent.ComponentTags` _bp_vent))))

(fn `UserConstructionScript`)